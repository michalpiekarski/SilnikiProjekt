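; Base enemy ship for a twin-stick shooter that flies along its forward axis and dies when hit by a player projectile.
; A hit stops shooting and adds its score value through the player controller.
; If its position projects to screen, it hides, may spawn a random-type pickup, and floats a score widget upward via a timeline before removal.
; The construction script applies the configurable ship mesh.
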(event OnComponentBeginOverlap(ShipMesh)
  (params (OtherActor :type Actor%20Object%20Reference) (OtherComp :type Primitive%20Component%20Object%20Reference) (OtherBodyIndex :type Integer) (bFromSweep :type Boolean) (SweepResult :type Hit%20Result%20Structure%20%28by%20ref%29))
  (bind _returnvalue (Game|GetPlayerController 0))
  (bind _shipmesh (Variables|Default|GetShipMesh))
  (bind _returnvalue_2 (Transformation|GetWorldLocation _shipmesh))
  (bind (_screenlocation _returnvalue_3) (Class|PlayerController|ProjectWorldLocationtoScreen _returnvalue _returnvalue_2))
  ;[1 1 1] Destroy On Contact With Projectile
  (Utilities|Casting|CastToTwinStickProjectile OtherActor)
  (Variables|WeaponSystem|SetCanShoot false)
  (|UpdateScore)
  (if _returnvalue_3
    (Variables|UI|SetShipDeathLocationInScreen _screenlocation)
    (Rendering|SetVisibility (Variables|Default|GetShipMesh) false false)
    (Collision|SetCollisionEnabled (Variables|Default|GetShipMesh) "NoCollision")
    (if (< (Math|Random|RandomIntegerinRange 1 100) 25)
      (|PickUpSpawn_2))
    (|ShowAndAnimateTheScoreValueText
      (:Finished
        _)))
  (Actor|DestroyActor))

(event EventTick
  (params (DeltaSeconds :type Float%20%28single-precision%29))
  ;[1 1 1] Move Forward
  (Transformation|AddRelativeLocation (Variables|Default|GetShipMesh) (* (* (Math|Vector|GetForwardVector (Variables|Default|GetTransform)) -1.0) (Variables|Mobility|GetSpeed)) true))

(fn ConstructionScript
  (Components|StaticMesh|SetStaticMesh (Variables|Default|GetShipMesh) (Variables|Rendering|GetShipModel)))