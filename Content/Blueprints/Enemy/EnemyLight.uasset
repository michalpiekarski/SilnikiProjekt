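; EnemyLight is a light enemy Blueprint that fires bullets from twin guns.
; On BeginPlay it starts FireTimeline, whose Fire event spawns a damage-carrying EnemyBullet at both the left and right gun transforms while CanShoot is true.
; When CanShoot is false at a Fire event, the timeline stops, and nothing in this graph restarts it.
; The construction script only calls its parent.
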(event EventBeginPlay
  (Timeline|FireTimeline PlayFromStart
    (:Fire
      (if (Variables|Default|GetCanShoot)
        (Game|SpawnActorfromClass "/Game/Blueprints/Enemy/EnemyBullet.EnemyBullet_C" (Transformation|GetWorldTransform (Variables|WeaponSystem|GetGunLeft)) false 2.5 0)
        (Game|SpawnActorfromClass "/Game/Blueprints/Enemy/EnemyBullet.EnemyBullet_C" (Transformation|GetWorldTransform (Variables|WeaponSystem|GetGunRight)) false 2.5 0)
        (else
          (Timeline|FireTimeline Stop))))))

(fn ConstructionScript
  (|CallParentFunction))