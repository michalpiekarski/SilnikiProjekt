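; EnemyHeavy is a multi-gun enemy that fires EnemyBullet actors in a timed pattern.
; On BeginPlay it starts FireTimeline, whose three event tracks trigger the outer pair, inner pair and center gun.
; Each shot spawns a bullet at that gun component's world transform, with helper functions handling the left and right pairs.
; The construction script only calls its parent.
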(event EventBeginPlay
  (Timeline|FireTimeline PlayFromStart
    (:FireOut
      (|FireOutGuns))
    (:FireIn
      (|FireInGuns))
    (:FireCenter
      (Game|SpawnActorfromClass "/Game/Blueprints/Enemy/EnemyBullet.EnemyBullet_C" (Transformation|GetWorldTransform (Variables|Default|GetGunCenter)) false 0))))

(fn ConstructionScript
  (|CallParentFunction))