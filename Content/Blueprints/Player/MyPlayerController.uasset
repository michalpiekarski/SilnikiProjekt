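; Player controller that owns the PlayerHUD, tracks score and kill count, and ramps global speed as kills accumulate.
; BeginPlay caches the pawn and builds the HUD; helper functions refresh its health, ammo and fuel bars, while a timeline animates the booster bar.
; SetScoreText updates score and increments EnemiesKilled on every call, including resets.
; Tick raises GlobalSpeedAcceleration when that count hits progressively wider-spaced thresholds.
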(event Custom|BoosterTurnedOn
  (bind _boosterpercent (Timeline|BoosterBarTimeline Play)
    (:Update
      (Progress|SetPercent (Variables|/Game/Blueprints/UI/PlayerHUD.PlayerHUD_C|GetBoosterBar (Variables|UI|GetCurrentHUD)) _boosterpercent))))

(event Custom|BoosterTurnedOff
  (bind _boosterpercent (Timeline|BoosterBarTimeline Reverse)
    (:Update
      (Progress|SetPercent (Variables|/Game/Blueprints/UI/PlayerHUD.PlayerHUD_C|GetBoosterBar (Variables|UI|GetCurrentHUD)) _boosterpercent))))

(event EventBeginPlay
  (CallFunction|SetCurrentPlayerPawn)
  (bind _returnvalue (UserInterface|CreateWidget (Variables|UI|GetPlayerHUD) self))
  (bind _asplayerhud_c (Utilities|Casting|CastToPlayerHUD _returnvalue))
  (Variables|UI|SetCurrentHUD _asplayerhud_c)
  (CallFunction|SetHealthBarPercent)
  (CallFunction|SetAmmoBarPercent)
  (CallFunction|SetFuelBarPercent)
  (CallFunction|SetScoreText 0 true)
  (UserInterface|Viewport|AddtoViewport (Variables|UI|GetCurrentHUD)))

(event EventTick
  (params (DeltaSeconds :type Float%20%28single-precision%29))
  (if (== (Variables|Gameplay|GetEnemiesKilled) (Variables|Gameplay|GetGlobalSpeedAccelerationStep))
    (Variables|Gameplay|SetGlobalSpeedAccelerationStep (+ (Variables|Gameplay|GetGlobalSpeedAccelerationStep) (Variables|Gameplay|GetGlobalSpeedAccelerationStepInrease)))
    (Variables|Gameplay|SetGlobalSpeedAccelerationStepInrease (+ (Variables|Gameplay|GetGlobalSpeedAccelerationStepInrease) 10))
    (Variables|Gameplay|SetGlobalSpeedAcceleration (+ (Variables|Gameplay|GetGlobalSpeedAcceleration) 5.0))))

(fn ConstructionScript)

(fn SetCurrentPlayerPawn
  (bind _asmyplayerpawn_c (Utilities|Casting|CastToMyPlayerPawn (Pawn|GetControlledPawn)))
  (Variables|Default|SetCurrentPlayerPawn _asmyplayerpawn_c))

(fn SetHealthBarPercent
  (bind _currentplayerpawn (Variables|Default|GetCurrentPlayerPawn))
  (Progress|SetPercent (Variables|/Game/Blueprints/UI/PlayerHUD.PlayerHUD_C|GetHealthBar (Variables|UI|GetCurrentHUD)) (/ (Variables|/Game/Blueprints/Player/MyPlayerPawn.MyPlayerPawn_C|GetHealth _currentplayerpawn) (Variables|/Game/Blueprints/Player/MyPlayerPawn.MyPlayerPawn_C|GetMaxHealth _currentplayerpawn))))

(fn SetAmmoBarPercent
  (bind _currentplayerpawn (Variables|Default|GetCurrentPlayerPawn))
  (Progress|SetPercent (Variables|/Game/Blueprints/UI/PlayerHUD.PlayerHUD_C|GetAmmoBar (Variables|UI|GetCurrentHUD)) (/ (Variables|/Game/Blueprints/Player/MyPlayerPawn.MyPlayerPawn_C|GetAmmo _currentplayerpawn) (Variables|/Game/Blueprints/Player/MyPlayerPawn.MyPlayerPawn_C|GetMaxAmmo _currentplayerpawn))))

(fn SetScoreText
  (params (Points :type Integer) (Reset :type Boolean))
  (if Reset
    (Variables|Gameplay|SetScore 0)
    (else
      (Variables|Gameplay|SetScore (+ Points (Variables|Gameplay|GetScore)))))
  (Rendering|Components|TextRender|SetText (Variables|/Game/Blueprints/UI/PlayerHUD.PlayerHUD_C|GetScoreText (Variables|UI|GetCurrentHUD)) (Utilities|Text|ToText(String) (Utilities|String|Append "SCORE: " (Utilities|String|ToString(Integer) (Variables|Gameplay|GetScore)))))
  (Variables|Gameplay|SetEnemiesKilled (+ (Variables|Gameplay|GetEnemiesKilled) 1)))

(fn SetFuelBarPercent
  (bind _currentplayerpawn (Variables|Default|GetCurrentPlayerPawn))
  (Progress|SetPercent (Variables|/Game/Blueprints/UI/PlayerHUD.PlayerHUD_C|GetFuelBar (Variables|UI|GetCurrentHUD)) (/ (Variables|/Game/Blueprints/Player/MyPlayerPawn.MyPlayerPawn_C|GetFuel _currentplayerpawn) (Variables|/Game/Blueprints/Player/MyPlayerPawn.MyPlayerPawn_C|GetMaxFuel _currentplayerpawn))))