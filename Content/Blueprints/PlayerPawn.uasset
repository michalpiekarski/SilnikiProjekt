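; PlayerPawn is a player-controlled ship pawn that handles movement, boosting and shooting.
; Axis inputs move ShipMesh by swept relative offsets scaled by Speed, which the Booster input multiplies while held.
; Fire input starts a timeline unless one is playing; its event track spawns TwinStickProjectile actors from center, left and right guns.
; Each shot plays FireSound at the world origin, and the firing logic is marked temporary.
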(event Input|ActionEvents|InputActionBooster
  (bind _boosterspeedmultiplier (Variables|Mobility|GetBoosterSpeedMultiplier))
  ;[1 1 1] Sterowanie lotem
  (:Pressed
    (Variables|Mobility|SetSpeed (* (Variables|Mobility|GetSpeed) _boosterspeedmultiplier)))
  (:Released
    (Variables|Mobility|SetSpeed (/ (Variables|Mobility|GetSpeed) _boosterspeedmultiplier))))

(event Input|ActionEvents|InputActionFire
  ;[1 1 1] Fire - TEMP
  (:Pressed
    (if (not (Audio|Components|Audio|IsPlaying (Variables|Default|GetFireTimeline)))
      (Timeline|FireTimeline PlayFromStart
        (:Fire
          (CallFunction|Fire (Variables|WeaponSystem|GetGunCenter))
          (CallFunction|Fire (Variables|WeaponSystem|GetGunLeft))
          (CallFunction|Fire (Variables|WeaponSystem|GetGunRight)))))))

(event Input|AxisEvents|InputAxisMoveForward
  (params (AxisValue :type Float%20%28single-precision%29))
  ;[1 1 1] Sterowanie lotem
  (Transformation|AddRelativeLocation (Variables|Rendering|GetShipMesh) (Math|Vector|MakeVector (* AxisValue (Variables|Mobility|GetSpeed)) 0.0 0.0) true)
  (Math|Float|CompareFloat AxisValue 0.0))

(event Input|AxisEvents|InputAxisMoveRight
  (params (AxisValue :type Float%20%28single-precision%29))
  ;[1 1 1] Sterowanie lotem
  (Transformation|AddRelativeLocation (Variables|Rendering|GetShipMesh) (Math|Vector|MakeVector 0.0 (* AxisValue (Variables|Mobility|GetSpeed)) 0.0) true)
  (Math|Float|CompareFloat AxisValue 0.0))

(fn ConstructionScript)

(fn Fire
  (params (Gun :type Scene%20Component%20Object%20Reference))
  (Game|SpawnActorfromClass "/Game/Blueprints/TwinStickProjectile.TwinStickProjectile_C" (Transformation|GetWorldTransform Gun) false 0)
  (Audio|PlaySoundatLocation (Variables|Audio|GetFireSound) "0, 0, 0"))