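; Enemy spawn volume that repeatedly spawns a configurable actor class at random points within its box.
; The construction script caches the box's scaled extents, world location and rotation.
; A looping timer started on BeginPlay calls Spawn, which picks a random offset and uniform random scale and uses the box's rotation for the spawned actor.
; Offsets are world-axis aligned, ignoring box rotation, and spawns are skipped when colliding.
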(event EventBeginPlay
  (Utilities|Time|SetTimerbyFunctionName 0 "Spawn" (Variables|Default|GetSpawnDelay) true))

(fn ConstructionScript
  (bind _returnvalue (Transformation|GetActorScale3D))
  (bind _box1 (Variables|Default|GetBox1))
  (bind _boxextent (Variables|/Script/Engine.BoxComponent|GetBoxExtent _box1))
  (bind _returnvalue_2 (* _boxextent _returnvalue))
  (bind (_x _y _z) (Math|Vector|BreakVector _returnvalue_2))
  (Variables|Default|SetMaxExX _x)
  (Variables|Default|SetMinExX (* _x -1.0))
  (Variables|Default|SetMaxExY _y)
  (Variables|Default|SetMinExY (* _y -1.0))
  (Variables|Default|SetMaxExZ _z)
  (Variables|Default|SetMinExZ (* _z -1.0))
  (Variables|Default|SetLoc (Transformation|GetWorldLocation _box1))
  (Variables|Default|SetRot (Transformation|GetWorldRotation _box1)))

(fn Spawn
  (Game|SpawnActorfromClass (Variables|Default|GetSpawnTarget) (Math|Transform|MakeTransform (+ (Math|Vector|MakeVector (Math|Random|RandomFloatinRange (Variables|Default|GetMinExX) (Variables|Default|GetMaxExX)) (Math|Random|RandomFloatinRange (Variables|Default|GetMinExY) (Variables|Default|GetMaxExY)) (Math|Random|RandomFloatinRange (Variables|Default|GetMinExZ) (Variables|Default|GetMaxExZ))) (Variables|Default|GetLoc)) (Variables|Default|GetRot) (* (Math|Vector|MakeVector 1.0 1.0 1.0) (Math|Random|RandomFloatinRange (Variables|Default|GetMinSpawnScale) (Variables|Default|GetMaxSpawnScale)))) false))