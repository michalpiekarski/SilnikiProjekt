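; Pickup actor that the player pawn collects by overlapping its trigger, with a type of health, fuel, ammo or score multiplier.
; On overlap it broadcasts the event dispatcher matching its type, leaving the actual reward to listeners.
; It then activates its effect, plays an explosion sound at the world origin rather than its own location, and destroys itself after a short delay.
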(event OnComponentBeginOverlap(PickUpTrigger)
  (params (OtherActor :type Actor%20Object%20Reference) (OtherComp :type Primitive%20Component%20Object%20Reference) (OtherBodyIndex :type Integer) (bFromSweep :type Boolean) (SweepResult :type Hit%20Result%20Structure%20%28by%20ref%29))
  (Utilities|Casting|CastToMyPlayerPawn OtherActor)
  (switch Utilities|FlowControl|Switch|SwitchonPickUpEnum (Variables|Default|GetPickUpType)
    (:NewEnumerator0
      (Default|CallHealthPick))
    (:NewEnumerator1
      (Default|CallFuelPick))
    (:NewEnumerator2
      (Default|CallAmmoPick))
    (:NewEnumerator3
      (Default|CallScoreMulPick)))
  (Components|Activation|Activate (Variables|Default|GetPickUpEffect) false)
  (Audio|PlaySoundatLocation "/Game/StarterContent/Audio/Explosion01.Explosion01" "0, 0, 0")
  (Utilities|FlowControl|Delay 0.3)
  (Actor|DestroyActor))

(fn ConstructionScript)