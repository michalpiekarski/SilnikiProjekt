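; EnemyShip is an enemy ship actor that flies steadily and is destroyed when hit by a twin-stick projectile.
; Each tick it sweeps StaticMesh1 along the negated forward vector by Speed, with no delta-time scaling, so movement depends on frame rate.
; An overlap on that mesh destroys the actor only if the other actor casts to TwinStickProjectile.
; The construction script applies a hex tile material to the mesh.
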(event OnComponentBeginOverlap(StaticMesh1)
  (params (OtherActor :type Actor%20Object%20Reference) (OtherComp :type Primitive%20Component%20Object%20Reference) (OtherBodyIndex :type Integer) (bFromSweep :type Boolean) (SweepResult :type Hit%20Result%20Structure%20%28by%20ref%29))
  (Utilities|Casting|CastToTwinStickProjectile OtherActor)
  (Actor|DestroyActor))

(event EventTick
  (params (DeltaSeconds :type Float%20%28single-precision%29))
  (Transformation|AddRelativeLocation (Variables|Default|GetStaticMesh1) (* (* (Math|Vector|GetForwardVector (Variables|Default|GetTransform)) -1.0) (Variables|Default|GetSpeed)) true))

(fn ConstructionScript
  (Rendering|Material|SetMaterial (Variables|Default|GetStaticMesh1) 0 "/Game/StarterContent/Materials/M_Tech_Hex_Tile.M_Tech_Hex_Tile"))