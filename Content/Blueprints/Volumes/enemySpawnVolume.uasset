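; Enemy spawn volume that spawns random enemy types in timed waves inside its box.
; BeginPlay sets a timer that toggles a repeating Spawn timer every WaveDuration, alternating pauses and waves, starting with a pause.
; In SingleWave mode the toggle timer fires once, and a delayed second toggle ends the wave.
; Each spawn picks a random class from EnemyTypes and a random location and uniform scale, using the box's rotation.
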(event EventBeginPlay
  (Utilities|Time|SetTimerbyFunctionName 0 "ToggleSpawn" (Variables|Default|GetWaveDuration) (not (Variables|Default|GetSingleWave)))
  (if (Variables|Default|GetSingleWave)
    (Utilities|FlowControl|Delay (* (Variables|Default|GetWaveDuration) 2.0))
    (CallFunction|ToggleSpawn)))

(fn ConstructionScript)

(fn Spawn
  (Game|SpawnActorfromClass (|GetRandomEnemyType) (|GetRandomSpawnLocation) false 0))

(fn ToggleSpawn
  (if (Class|KismetSystemLibrary|IsTimerActive 0 "Spawn")
    (Utilities|Time|ClearTimerbyFunctionName 0 "Spawn")
    (else
      (Utilities|Time|SetTimerbyFunctionName 0 "Spawn" (Variables|Default|GetSpawnDelay) true))))