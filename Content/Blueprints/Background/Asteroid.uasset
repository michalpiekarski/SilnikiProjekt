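; Asteroid hazard for what appears to be a twin-stick shooter, drifting forward while tumbling.
; The construction script randomizes its mesh, dynamic-material texture, speed and spin rates.
; Tick sweeps the box along its forward vector by Speed per frame, while rotation scales with delta time.
; Projectile or player overlap hides it, awards score, triggers explosion effects and destroys it after a delay, damaging the player first on contact.
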(event OnComponentBeginOverlap(Asteroid)
  (params (OtherActor :type Actor%20Object%20Reference) (OtherComp :type Primitive%20Component%20Object%20Reference) (OtherBodyIndex :type Integer) (bFromSweep :type Boolean) (SweepResult :type Hit%20Result%20Structure%20%28by%20ref%29))
  (bind _asteroid (Variables|Default|GetAsteroid))
  ;[1 1 1] Destroy on player and projectile hit
  (Utilities|Casting|CastToTwinStickProjectile OtherActor
    (:then
      _)
    (:CastFailed
      (bind _asmyplayerpawn_c (Utilities|Casting|CastToMyPlayerPawn OtherActor))
      (Default|TakeDamage _asmyplayerpawn_c 25.0)))
  (Collision|SetCollisionEnabled _asteroid "NoCollision")
  (Rendering|SetVisibility _asteroid false false)
  (bind _asmyplayercontroller_c (Utilities|Casting|CastToMyPlayerController (Game|GetPlayerController 0)))
  (Default|SetScoreText _asmyplayercontroller_c 25 false)
  (Components|Activation|SetActive (Variables|Default|GetBoom) true false)
  (Audio|PlaySoundatLocation "/Game/StarterContent/Audio/Explosion01.Explosion01" "0, 0, 0")
  (Utilities|FlowControl|Delay 1.0)
  (Actor|DestroyActor))

(event EventTick
  (params (DeltaSeconds :type Float%20%28single-precision%29))
  (bind _box1 (Variables|Default|GetBox1))
  ;[1 1 1] Move Forward and Spin
  (Transformation|AddRelativeLocation _box1 (* (Math|Vector|GetForwardVector _box1) (Variables|Default|GetSpeed)) true)
  (Transformation|AddWorldRotation (Variables|Default|GetAsteroid) (Class|KismetMathLibrary|MakeRot (* DeltaSeconds (Variables|Default|GetPitch)) (* DeltaSeconds (Variables|Default|GetYaw)) (* DeltaSeconds (Variables|Default|GetRoll))) false))

(fn ConstructionScript
  (bind _returnvalue (Math|Random|RandomFloatinRange 1e+01 1e+02))
  (bind _asteroid (Variables|Default|GetAsteroid))
  (bind _returnvalue_2 (Rendering|Material|CreateDynamicMaterialInstance "/Game/Materials/Asteroids_material.Asteroids_material" :!class /Script/Engine.KismetMaterialLibrary))
  (Rendering|Material|SetTextureParameterValue _returnvalue_2 "RandomTexture" (Utilities|Array|Get(acopy) (Variables|Default|GetRandTextureArray) (Math|Random|RandomIntegerinRange 0 5)))
  (Rendering|Material|SetMaterial _asteroid 0 _returnvalue_2)
  (Components|StaticMesh|SetStaticMesh _asteroid (Utilities|Array|Get(acopy) (Variables|Default|GetRandMeshArray) (Math|Random|RandomIntegerinRange 0 5)))
  (Variables|Default|SetSpeed (Math|Random|RandomFloatinRange 5.0 3e+01))
  (Variables|Default|SetPitch _returnvalue)
  (Variables|Default|SetYaw _returnvalue)
  (Variables|Default|SetRoll _returnvalue))